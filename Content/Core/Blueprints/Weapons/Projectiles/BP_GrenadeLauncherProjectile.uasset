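; Grenade launcher projectile Blueprint that supplies the trail and explosion effects for the launched grenade.
; On BeginPlay it attaches a trail emitter to the collision component and stores it as the tracer component.
; OnExplode plays the explosion sound and spawns the explosion emitter at the actor's location, using assets returned by getter functions.
; A debug path drawing of spheres and lines is left disconnected, though the construction script still seeds its last location.
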(event `self.ReceiveBeginPlay`
  (bind _returnvalue (`GameplayStatics.SpawnEmitterAttached` (`Projectile.GetTrailEffect`) (`self.CollisionComp`) "None" (`self.K2_GetActorLocation`) (struct) (1.0 1.0 1.0) "KeepWorldPosition"))
  (set `self.TracerComponent` _returnvalue))

(event `self.OnExplode`
  (params (physicalMaterial :type "PhysicalMaterialBase Object Reference"))
  (bind _returnvalue (`self.K2_GetActorLocation`))
  (`GameplayStatics.PlaySoundAtLocation` (`Projectile.GetExplosionSound`) _returnvalue (struct) 1.0 1.0 0.0 null null null null)
  (`GameplayStatics.SpawnEmitterAtLocation` (`Projectile.GetExplosionEffect`) _returnvalue))

(event `self.ReceiveTick`
  (params (DeltaSeconds :type "Float (single-precision)")))

(fn `UserConstructionScript`
  (set `self.LastProjectileLocation` (`self.K2_GetActorLocation`)))