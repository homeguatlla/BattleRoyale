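; Assault rifle bullet projectile Blueprint that handles the round's trail and impact feedback.
; On BeginPlay it attaches the trail emitter to the collision component and stores it as the tracer component.
; On explode, if the physical material has a valid impact sound, it plays that sound and spawns the explosion effect at the bullet's location.
; Debug drawing of the flight path is present but disconnected.
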(event `self.ReceiveBeginPlay`
  (bind _returnvalue (`GameplayStatics.SpawnEmitterAttached` (`Projectile.GetTrailEffect`) (`self.CollisionComp`) "None" (`self.K2_GetActorLocation`) (`self.K2_GetActorRotation`) (1.0 1.0 1.0) "KeepWorldPosition"))
  (set `self.TracerComponent` _returnvalue))

(event `self.OnExplode`
  (params (physicalMaterial :type "PhysicalMaterialBase Object Reference"))
  (bind _returnvalue (`self.K2_GetActorLocation`))
  (bind _impactsound (`PhysicalMaterialBase.ImpactSound` physicalMaterial))
  (`/Engine/EditorBlueprintResources/StandardMacros.IsValid` physicalMaterial
    (:`Is Valid`
      (`/Engine/EditorBlueprintResources/StandardMacros.IsValid` _impactsound
        (:`Is Valid`
          (`GameplayStatics.PlaySoundAtLocation` _impactsound _returnvalue (struct) 1.0 1.0 0.0 null null null null)
          (`GameplayStatics.SpawnEmitterAtLocation` (`Projectile.GetExplosionEffect`) _returnvalue))))))

(event `self.ReceiveTick`
  (params (DeltaSeconds :type "Float (single-precision)")))

(fn `UserConstructionScript`
  (set `self.LastProjectileLocation` (`self.K2_GetActorLocation`)))