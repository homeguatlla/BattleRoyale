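; BP_AssaultRifle is an assault rifle weapon Blueprint that adds sound feedback to weapon events.
; Equip and ammo-in events play the raise cue, reload plays the reload cue, and ammo-out plays the lower cue.
; OnFire only handles the empty case, playing the lower cue when HasAmmo is false.
; All sounds play at the actor's location, and the construction script is empty.
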(event `self.BP_OnEquipped`
  (`GameplayStatics.PlaySoundAtLocation` "/Game/Weapons/AssaultRifle/Sounds/Cues/Rifle_Raise_Cue.Rifle_Raise_Cue" (`self.K2_GetActorLocation`) (struct) 1.0 1.0 0.0 null null null null))

(event `self.BP_OnFire`
  ;[1 1 1] If no ammo when firing, trigger sound
  (if (not (`Weapon.HasAmmo`))
    (`GameplayStatics.PlaySoundAtLocation` "/Game/Weapons/AssaultRifle/Sounds/Cues/Rifle_Lower_Cue.Rifle_Lower_Cue" (`self.K2_GetActorLocation` self) (struct) 1.0 1.0 0.0 null null null null)))

(event `self.BP_OnReload`
  (`GameplayStatics.PlaySoundAtLocation` "/Game/Weapons/AssaultRifle/Sounds/Cues/Rifle_Reload_Cue.Rifle_Reload_Cue" (`self.K2_GetActorLocation`) (struct) 1.0 1.0 0.0 null null null null))

(event `self.BP_OnReloadAmmoIn`
  (`GameplayStatics.PlaySoundAtLocation` "/Game/Weapons/AssaultRifle/Sounds/Cues/Rifle_Raise_Cue.Rifle_Raise_Cue" (`self.K2_GetActorLocation`) (struct) 1.0 1.0 0.0 null null null null))

(event `self.BP_OnReloadAmmoOut`
  (`GameplayStatics.PlaySoundAtLocation` "/Game/Weapons/AssaultRifle/Sounds/Cues/Rifle_Lower_Cue.Rifle_Lower_Cue" (`self.K2_GetActorLocation`) (struct) 1.0 1.0 0.0 null null null null))

(fn `UserConstructionScript`)