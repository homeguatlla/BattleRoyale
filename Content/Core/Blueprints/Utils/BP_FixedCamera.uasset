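; Debug utility that lets the player toggle the view between a fixed camera and the controlled pawn.
; The C key flip-flops SetViewTargetWithBlend between the two with one-second blends and sets IsCameraTraceShown, which B also toggles.
; Tick checks that flag but does nothing, leaving DebugDrawCameraDirection disconnected.
; That function traces along the pawn's control rotation on the Camera channel and draws the line and spheres.
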(event `Key|C`
  (params (Key :type "Key Structure"))
  (bind _returnvalue (`GameplayStatics.GetPlayerController` 0))
  (:`Pressed`
    (`/Engine/EditorBlueprintResources/StandardMacros.FlipFlop`
      (:`A`
        (set `self.isCameraTraceShown` true)
        (`PlayerController.SetViewTargetWithBlend` (`GameplayStatics.GetPlayerController` 0) (`self.FixedCamera`) 1.0 "VTBlend_EaseInOut" 2.0 true))
      (:`B`
        (set `self.isCameraTraceShown` false)
        (`PlayerController.SetViewTargetWithBlend` _returnvalue (`Controller.K2_GetPawn` _returnvalue) 1.0 "VTBlend_Cubic" 3.0 true)))))

(event `Key|B`
  (params (Key :type "Key Structure"))
  (:`Pressed`
    (bind _isa (`/Engine/EditorBlueprintResources/StandardMacros.FlipFlop`)
      (:`A`
        _)
      (:`B`
        _))
    (set `self.isCameraTraceShown` _isa)))

(event `self.ReceiveTick`
  (params (DeltaSeconds :type "Float (single-precision)"))
  (if (`self.isCameraTraceShown`)
    _))

(fn `DebugDrawCameraDirection`
  (bind _returnvalue (`Controller.K2_GetPawn` (`GameplayStatics.GetPlayerController` 0)))
  (bind _returnvalue_2 (`self.K2_GetActorLocation` _returnvalue))
  (`KismetSystemLibrary.DrawDebugSphere` _returnvalue_2 20.0)
  (bind _outhit (`KismetSystemLibrary.LineTraceSingle` _returnvalue_2 (+ (* (`KismetMathLibrary.GetForwardVector` (`Pawn.GetControlRotation` _returnvalue)) 3000.0) _returnvalue_2) "TraceTypeQuery2"))
  (`KismetSystemLibrary.DrawDebugLine` _returnvalue_2 (`.Location` (`GameplayStatics.BreakHitResult` _outhit)) (struct :`R` 1.0 :`G` 1.0 :`B` 1.0 :`A` 0.5))
  (`KismetSystemLibrary.DrawDebugSphere` (`.Location` (`GameplayStatics.BreakHitResult` _outhit)) 10.0))

(fn `UserConstructionScript`)