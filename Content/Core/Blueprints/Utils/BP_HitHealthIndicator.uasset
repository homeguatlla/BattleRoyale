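; BP_HitHealthIndicator is a floating text actor, apparently for hit or health feedback, that rises above a target and then destroys itself.
; The construction script sets the text, and BeginPlay applies the color and scales the MoveUp timeline's play rate to the set duration.
; Each timeline update re-reads the target's location and adds a curve-driven vertical offset scaled by MaxHeight, so the text follows the target.
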(event `self.ReceiveBeginPlay`
  (`TextRenderComponent.SetTextRenderColor` (`self.TextRender`) (`self.Color`))
  (`TimelineComponent.SetPlayRate` (`self.MoveUp`) (/ 1.0 (`self.Duration`)))
  (bind (_direction _height) (`Timeline|MoveUp` :!via `PlayFromStart`)
    (:`Update`
      (`self.K2_SetActorLocation` (+ (`ICharacter.GetLocation` (`self.Target`)) (`KismetMathLibrary.MakeVector` 0.0 0.0 (* _height (`self.MaxHeight`))))))
    (:`Finished`
      (`self.K2_DestroyActor`))))

(fn `UserConstructionScript`
  (`TextRenderComponent.K2_SetText` (`self.TextRender`) (`self.Text`)))