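; Gameplay ability that shows and hides a floating "E-Pick Up" prompt actor at a given location.
; The show event spawns the indicator once, then moves and reuses it, starting a looping timer that refreshes its transform about every frame.
; CalculateTransformation builds a yaw-only look-at toward the avatar actor so the prompt faces the player.
; The hide event hides the indicator and clears the timer.
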(event `self.OnShowPickupIndicator`
  (params (Location :type "Vector Structure (by ref)"))
  (bind _pickupindicator (`self.PickupIndicator`))
  (bind _output_get (set `self.Location` Location))
  (`/Engine/EditorBlueprintResources/StandardMacros.IsValid` _pickupindicator
    (:`Is Valid`
      (`Actor.K2_SetActorLocation` _pickupindicator Location false false))
    (:`Is Not Valid`
      (bind _returnvalue (`|SpawnActorFromClass` "/Game/Core/Blueprints/Utils/BP_PickupIndicator.BP_PickupIndicator_C" (`self.CalculateTransformation` _output_get) "Undefined" "OverrideRootScale" null "E-Pick Up" (struct :`B` 255 :`G` 255 :`R` 255 :`A` 255) null))
      (set `self.PickupIndicator` _returnvalue)))
  (bind _returnvalue_2 (`KismetSystemLibrary.K2_SetTimer` null "RefreshPickupRotation" 0.016 true))
  (set `self.RefreshTimer` _returnvalue_2)
  (`/Game/Core/Blueprints/Utils/BP_PickupIndicator.SetVisibility` (`self.PickupIndicator`) true))

(event `self.OnHidePickupIndicator`
  (`/Game/Core/Blueprints/Utils/BP_PickupIndicator.SetVisibility` (`self.PickupIndicator`) false)
  (`KismetSystemLibrary.K2_ClearAndInvalidateTimerHandle` (`self.RefreshTimer`)))

(fn `RefreshPickupRotation`
  (`Actor.K2_SetActorTransform` (`self.PickupIndicator`) (`self.CalculateTransformation` (`self.Location`)) false false))