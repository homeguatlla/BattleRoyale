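; Gameplay ability for a smoke skill that throws three smoke grenades from the avatar.
; On activation it commits, then the authority spawns the grenades in a short delayed loop and ends the ability.
; Each grenade spawns just ahead of the avatar with a fixed smoke duration.
; An impulse on its collider launches it toward a random upper-sector point around a spot ahead, set by Distance and Radius, scattering the throw.
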(event `self.K2_ActivateAbility`
  (`self.K2_CommitAbility`)
  (set `self.NumSmokesGrenades` 3)
  (if (`Actor.HasAuthority` (`self.GetAvatarActorFromActorInfo`))
    (if (> (`self.NumSmokesGrenades`) 0) :!label _label
      (`self.SpawnSmokeGrenade`)
      (`KismetSystemLibrary.Delay` 0.05)
      (set `self.NumSmokesGrenades` (- (`self.NumSmokesGrenades`) 1))
      (goto _label)
      (else
        (`self.K2_EndAbility`)))))

(event `self.K2_OnEndAbility`
  (params (bWasCancelled :type Boolean)))

(fn `SpawnSmokeGrenade`
  (bind _returnvalue (`self.GetAvatarActorFromActorInfo`))
  (bind _returnvalue_2 (`Actor.K2_GetActorLocation` _returnvalue))
  (bind _returnvalue_3 (`Actor.GetActorForwardVector` _returnvalue))
  (bind _returnvalue_4 (`|SpawnActorFromClass` "/Game/Core/Blueprints/Test/A_SmokeGrenade.A_SmokeGrenade_C" (`KismetMathLibrary.Conv_VectorToTransform` (+ _returnvalue_2 (* _returnvalue_3 50.0))) "AdjustIfPossibleButDontSpawnIfColliding" "MultiplyWithRoot" null 10.0 null))
  (`PrimitiveComponent.AddImpulse` (`/Game/Core/Blueprints/Test/A_SmokeGrenade.Collider` _returnvalue_4) (- (`GameplayBlueprintFunctionLibrary.GenerateRandomPointAtDistanceOf` (+ _returnvalue_2 (* _returnvalue_3 (`self.Distance`))) (`self.Radius`) true) _returnvalue_2) "None" false))