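; Gameplay ability that shows a floating name indicator and pulsing glow on a pickup object.
; On show, it spawns or reuses BP_PickupIndicator halfway between the mesh top and player eye height, then applies a dynamic glow material.
; A looping timer updates the indicator's transform to face the player and drives the glow with a sine wave.
; Hiding conceals the indicator, clears the timer and zeroes the glow.
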(event `self.OnShowPickupIndicator`
  (params (object :type "PickableObjectBase Object Reference") (Location :type "Vector Structure (by ref)"))
  (bind _pickupindicator (`self.PickupIndicator`))
  (bind _pickupindicator_2 (`self.PickupIndicator`))
  (bind _returnvalue (`KismetTextLibrary.Conv_NameToText` (`PickableObjectBase.GetPickableName` object)))
  (bind _location (`self.Calculate Indicator Location` object))
  (bind _z (`self.Calculate Player Eyes Z`))
  (bind _returnvalue_2 (* (- _z (.z _location)) 0.5))
  (bind _output_get (set `self.Location` (`KismetMathLibrary.MakeVector` (.x _location) (.y _location) (+ (.z _location) _returnvalue_2))))
  (`/Engine/EditorBlueprintResources/StandardMacros.IsValid` _pickupindicator
    (:`Is Valid`
      (set `self.Time` 0.0)
      (`Actor.K2_SetActorLocation` _pickupindicator _output_get false false))
    (:`Is Not Valid`
      (bind _returnvalue_3 (`|SpawnActorFromClass` "/Game/Core/Blueprints/Utils/BP_PickupIndicator.BP_PickupIndicator_C" (`self.CalculateTransformation` _output_get) "Undefined" "OverrideRootScale" null _returnvalue (struct :`G` 183 :`R` 251 :`A` 255) null))
      (set `self.PickupIndicator` _returnvalue_3)))
  (bind _returnvalue_4 (`PrimitiveComponent.CreateDynamicMaterialInstance` (`PickableObjectBase.GetMesh` object) 0 "/Game/Weapons/Materials/MI_WeaponMasterGlow.MI_WeaponMasterGlow" "None"))
  (set `self.GlowMaterialInstance` _returnvalue_4)
  (bind _returnvalue_5 (`KismetSystemLibrary.K2_SetTimer` null "RefreshPickupRotationAndObjectGlow" 0.016 true))
  (set `self.RefreshTimer` _returnvalue_5)
  (`/Game/Core/Blueprints/Utils/BP_PickupIndicator.SetVisibility` _pickupindicator_2 true)
  (`/Game/Core/Blueprints/Utils/BP_PickupIndicator.Refresh` _pickupindicator_2 (`self.Location`) _returnvalue_2 _returnvalue))

(event `self.OnHidePickupIndicator`
  (bind _pickupindicator (`self.PickupIndicator`))
  (bind _glowmaterialinstance (`self.GlowMaterialInstance`))
  (`|ExecutionSequence`
    (:`then_0`
      (`/Engine/EditorBlueprintResources/StandardMacros.IsValid` _pickupindicator
        (:`Is Valid`
          (`/Game/Core/Blueprints/Utils/BP_PickupIndicator.SetVisibility` _pickupindicator false)
          (`KismetSystemLibrary.K2_ClearAndInvalidateTimerHandle` (`self.RefreshTimer`)))))
    (:`then_1`
      (`/Engine/EditorBlueprintResources/StandardMacros.IsValid` _glowmaterialinstance
        (:`Is Valid`
          (`MaterialInstanceDynamic.SetScalarParameterValue` _glowmaterialinstance "Glow" 0.0))))))

(fn `Calculate Indicator Location`
  (params (pickupObject :type "PickableObjectBase Object Reference"))
  (returns (Location :type "Vector Structure"))
  (bind (_origin _boxextent) (`KismetSystemLibrary.GetComponentBounds` (`PickableObjectBase.GetMesh` pickupObject)))
  (bind _output_get (set `self.Box Extent` _boxextent))
  (return (+ _origin (`KismetMathLibrary.MakeVector` 0.0 0.0 (.z _output_get)))))

(fn `Calculate Player Eyes Z`
  (returns (Z :type "Float (double-precision)"))
  (bind (_origin _boxextent) (`KismetSystemLibrary.GetComponentBounds` (`Character.Mesh` (`GameplayStatics.GetPlayerCharacter` 0))))
  (return (- (+ (.z _origin) (.z _boxextent)) 30.0)))

(fn `RefreshPickupRotationAndObjectGlow`
  ;[1 1 1] Update rotation to the player on the text 3D
  (`Actor.K2_SetActorTransform` (`self.PickupIndicator`) (`self.CalculateTransformation` (`self.Location`)) false false)
  ;[1 1 1] Change object glow
  (bind _output_get (set `self.Time` (+ (`self.Time`) 0.05)))
  (`MaterialInstanceDynamic.SetScalarParameterValue` (`self.GlowMaterialInstance`) "Glow" (* (`KismetMathLibrary.Sin` _output_get) 300.0)))